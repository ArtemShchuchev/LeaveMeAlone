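; PC_LeaveMeAlone is a player controller Blueprint that opens the pause menu when the Pause input is pressed.
; If not already paused, it sets the OnPause flag, calls FireEnd on the pawn's LMAWeaponComponent and pauses the game.
; It then creates and displays WBP_Pause, switches to UI-only input focused on that widget and shows the mouse cursor.
; Nothing in this graph clears the flag or unpauses the game.
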(event EventTick
  (params (DeltaSeconds :type Float%20%28single-precision%29)))

(event Input|ActionEvents|InputActionPause
  (params (Key :type Key%20Structure :default "None"))
  (:Pressed
    (if (not (Variables|Default|GetOnPause))
      (Variables|Default|SetOnPause true)
      (Class|LMAWeaponComponent|FireEnd (Actor|GetComponentbyClass (Game|Player|GetPlayerPawn 0) "/Script/LeaveMeAlone.LMAWeaponComponent"))
      (Game|SetGamePaused true)
      (bind _returnvalue (UserInterface|CreateWidget "/Game/LeaveMeAlone/Widgets/UI/WBP_Pause.WBP_Pause_C"))
      (bind _output_get (Variables|Default|SetPauseWidget _returnvalue))
      (UserInterface|Viewport|AddtoViewport _output_get 0)
      (Input|SetInputModeUIOnly self _output_get "DoNotLock" false)
      (Variables|Default|SetbShowMouseCursor true))))

(fn ConstructionScript)